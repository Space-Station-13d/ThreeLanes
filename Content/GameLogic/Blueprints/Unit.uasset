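; Base unit for a turn-based grid game, registering its creation, destruction and turn end with TLGameState.
; Hit points start at maximum, change through damage and repair functions, and trigger destruction at zero.
; MoveForward recursively enters neighboring cells, decrementing but never testing Range, until another unit triggers the empty OnEncounterUnit event or the map edge destroys it.
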(event `self.ReceiveBeginPlay`
  (bind _astlgame_state (cast `/Game/GameLogic/TLGameState` (`GameplayStatics.GetGameState`)))
  (`/Game/GameLogic/TLGameState.On Unit Created` _astlgame_state self))

(event `self.ReceiveDestroyed`
  (bind _astlgame_state (cast `/Game/GameLogic/TLGameState` (`GameplayStatics.GetGameState`)))
  (`/Game/GameLogic/TLGameState.On Unit Destroyed` _astlgame_state self))

(event `On Turn Start`
  (set `self.Has Finished Turn` false))

(event `On Encounter Unit`
  (params (Unit :type "/Game/GameLogic/Blueprints/Unit Object Reference")))

(fn `Check Death`
  (if (not (> (`self.Hit Points`) 0))
    (`self.Die`)))

(fn `Die`
  (`self.K2_DestroyActor`))

(fn `End Turn`
  (set `self.Has Finished Turn` true)
  (bind _astlgame_state (cast `/Game/GameLogic/TLGameState` (`GameplayStatics.GetGameState`)))
  (`/Game/GameLogic/TLGameState.On Unit Ended Turn` _astlgame_state))

(fn `Enter Cell`
  (params (Cell :type "GridCell Object Reference"))
  (returns (Entered :type Boolean))
  (bind _cell (`self.Cell`))
  (`GridCell.SetCurrent` Cell (`self.Griddable`))
  (`KismetSystemLibrary.PrintText` (`|FormatText` "Unit {Unit} entered cell at X:{X} Y:{Y}." (`self.Name`) (`GridCell.X` _cell) (`GridCell.Y` _cell)))
  (return true))

(fn `Move Forward`
  (params (Direction :type "EGridNeighbor Enum") (Range :type Integer))
  (bind _returnvalue (`GridCell.GetNeighbor` (`self.Cell`) Direction))
  (bind _returnvalue_2 (`GridCell.GetCurrent` _returnvalue))
  (`/Engine/EditorBlueprintResources/StandardMacros.IsValid` _returnvalue
    (:`Is Valid`
      (`/Engine/EditorBlueprintResources/StandardMacros.IsValid` _returnvalue_2
        (:`Is Valid`
          (bind _asunit (cast `/Game/GameLogic/Blueprints/Unit` (`ActorComponent.GetOwner` _returnvalue_2)))
          (`self.On Encounter Unit` _asunit))
        (:`Is Not Valid`
          (bind _entered (`self.Enter Cell` _returnvalue))
          (if _entered
            (`self.Move Forward` Direction (- Range 1))))))
    (:`Is Not Valid`
      (`self.Try Exit Map`))))

(fn `Repair Damage`
  (params (Repair :type Integer))
  (set `self.Hit Points` (`KismetMathLibrary.Max` (+ Repair (`self.Hit Points`)) (`self.Max Hit Points`))))

(fn `Take Damage`
  (params (Damage :type Integer))
  (set `self.Hit Points` (`KismetMathLibrary.Max` Damage (- (`self.Hit Points`) Damage)))
  (`self.Check Death`))

(fn `Try Exit Map`
  (returns (Exited :type Boolean))
  (bind _cell (`self.Cell`))
  (`KismetSystemLibrary.PrintText` (`|FormatText` "Unit {Unit} exited map from X:{X} Y:{Y}." (`self.Name`) (`GridCell.X` _cell) (`GridCell.Y` _cell)))
  (`self.Die`)
  (return false))

(fn `UserConstructionScript`
  (set `self.Hit Points` (`self.Max Hit Points`)))
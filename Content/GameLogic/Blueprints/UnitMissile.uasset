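; UnitMissile is a turn-based projectile unit that travels across the map and damages the unit it runs into.
; At each turn start it calls the parent logic, then moves forward along its Direction with Speed as the range.
; On encountering a unit it applies its Damage and dies.
; It overrides TryExitMap to die and return true, so leaving the map also destroys it.
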(event `self.On Turn Start`
  (`parent.On Turn Start`)
  (`self.Move Forward` (`self.Direction`) (`self.Speed`)))

(event `self.On Encounter Unit`
  (params (Unit :type "/Game/GameLogic/Blueprints/Unit Object Reference"))
  (`parent.On Encounter Unit` Unit)
  (`self.Take Damage` Unit (`self.Damage`))
  (`self.Die`))

(fn `Try Exit Map`
  (returns (Exited :type Boolean))
  (`self.Die`)
  (return true))

(fn `UserConstructionScript`
  (`parent.UserConstructionScript`))
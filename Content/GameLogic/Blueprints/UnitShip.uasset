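; UnitShip is a ship unit Blueprint that manages an energy pool in a turn-based game.
; The construction script fills Energy to MaxEnergy, and each turn start restores EnergyRegen through GainEnergy, capped at the maximum.
; SpendEnergy deducts a cost only when enough energy is available and returns whether it succeeded.
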(event `self.On Turn Start`
  (`self.Gain Energy` (`self.Energy Regen`)))

(fn `Gain Energy`
  (params (Amount :type Integer))
  (set `self.Energy` (`KismetMathLibrary.Min` (+ Amount (`self.Energy`)) (`self.Max Energy`))))

(fn `Spend Energy`
  (params (Amount :type Integer))
  (returns (Spent :type Boolean))
  (if (<= Amount (`self.Energy`))
    (set `self.Energy` (- (`self.Energy`) Amount))
    (return true)
    (else
      (return false))))

(fn `UserConstructionScript`
  (`parent.UserConstructionScript`)
  (set `self.Energy` (`self.Max Energy`)))